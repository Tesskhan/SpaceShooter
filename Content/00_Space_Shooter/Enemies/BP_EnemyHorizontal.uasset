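; BP_EnemyHorizontal is a space shooter enemy variant that sets a sideways movement direction and reverses it at blockers.
; BeginPlay runs the parent logic, then sets MovementVector to the actor's right vector.
; On overlap with an actor tagged "Block", it negates that vector after calling the parent handler.
; It has no active Tick logic of its own, so this file only sets the direction.
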(event EventBeginPlay
  (|CallParentFunction)
  (Variables|Default|SetMovementVector (Transformation|GetActorRightVector)))

(event Collision|EventActorBeginOverlap
  (params (OtherActor :type Actor%20Object%20Reference))
  (|CallParentFunction OtherActor)
  (if (Utilities|Array|ContainsItem (Variables|/Script/Engine.Actor|GetTags OtherActor) "Block")
    (Variables|Default|SetMovementVector (Math|Vector|NegateVector (Variables|Default|GetMovementVector)))))

(event EventTick
  (params (DeltaSeconds :type Float%20%28single-precision%29))
  (|CallParentFunction DeltaSeconds) ; This node is disabled and will not be called.\nDrag off pins to build functionality.
)

(fn ConstructionScript
  (|CallParentFunction))